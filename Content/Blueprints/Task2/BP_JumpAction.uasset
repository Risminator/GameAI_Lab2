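; BP_JumpAction is an action that makes a controlled BP_BaseMannequin jump.
; On start it checks CanJump, finishing as failed if the jump is not possible.
; Otherwise it jumps, waits for an airtime computed from jump Z velocity and gravity, then finishes with success.
; The wait is a ballistic estimate that assumes landing at takeoff height, with no check for actual landing.
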(event EventActionStart
  (params (ControlledPawn :type Pawn%20Object%20Reference))
  (bind _asbp_base_mannequin (Utilities|Casting|CastToBP_BaseMannequin ControlledPawn))
  (if (Character|CanJump _asbp_base_mannequin)
    (Character|Jump _asbp_base_mannequin)
    (Utilities|FlowControl|Delay (/ (* 2 (Variables|/Script/Engine.CharacterMovementComponent|GetJumpZVelocity (Variables|/Script/Engine.Character|GetCharacterMovement _asbp_base_mannequin))) (Math|Float|Absolute(Float) (Components|Movement|GetGravityZ (Variables|/Script/Engine.Character|GetCharacterMovement _asbp_base_mannequin))))) ; Подождать завершения прыжка
    (FunctionalTesting|Finish "Success")
    (else
      (FunctionalTesting|Finish "Failed"))))
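; AI controller that walks its pawn in an endless loop through the BP_DestinationPoint actors in the level.
; On BeginPlay it gathers all destination points and issues AIMoveTo to the one at the current index.
; Each successful move advances the index with modulo wraparound and re-triggers the move through a GetToPoint event.
; Only the Success output is handled, so a failed move stops the loop.
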(event Custom|GetToPoint
  (bind _outactors (Actor|GetAllActorsOfClass "/Game/Blueprints/Task1/BP_DestinationPoint.BP_DestinationPoint_C"))
  (AI|AIMoveTo (Pawn|GetControlledPawn) "0, 0, 0" (Utilities|Array|Get(acopy) _outactors (Variables|Default|GetIndex_TP)) 5.0 false
    (:OnSuccess
      (bind _result (Math|Integer|IncrementInt (Variables|Default|GetIndex_TP))
        (:%20%20
          (Variables|Default|SetIndex_TP (Math|Integer|%(Integer) _result (Utilities|Array|Length _outactors)))
          (CallFunction|GettoPoint))))))

(event EventBeginPlay
  (bind _outactors (Actor|GetAllActorsOfClass "/Game/Blueprints/Task1/BP_DestinationPoint.BP_DestinationPoint_C"))
  (AI|AIMoveTo (Pawn|GetControlledPawn) "0, 0, 0" (Utilities|Array|Get(acopy) _outactors (Variables|Default|GetIndex_TP)) 5.0 false
    (:OnSuccess
      (bind _result (Math|Integer|IncrementInt (Variables|Default|GetIndex_TP))
        (:%20%20
          (Variables|Default|SetIndex_TP (Math|Integer|%(Integer) _result (Utilities|Array|Length _outactors)))
          (CallFunction|GettoPoint))))))

(fn ConstructionScript)
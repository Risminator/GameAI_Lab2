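; Behavior tree task that sends the AI-controlled pawn to one of the level's BP_DestinationPoint actors, selected by DestinationIndex.
; It gathers those actors with GetAllActorsOfClass, bounds-checks the index and runs AIMoveTo toward that entry, printing debug messages.
; Arrival finishes the task as a success and an invalid index as a failure.
; A failed move has no handler, so the task never finishes then.
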(event EventReceiveExecuteAI
  (params (OwnerController :type AI%20Controller%20Object%20Reference) (ControlledPawn :type Pawn%20Object%20Reference))
  (bind _destinationindex (Variables|Default|GetDestinationIndex))
  (bind _outactors (Actor|GetAllActorsOfClass "/Game/Blueprints/Task1/BP_DestinationPoint.BP_DestinationPoint_C"))
  (if (and (< _destinationindex (Utilities|Array|Length _outactors)) (>= _destinationindex 0))
    (AI|AIMoveTo ControlledPawn "0, 0, 0" (Utilities|Array|Get(acopy) _outactors _destinationindex) 5.0 false
      (:OnSuccess
        (Development|PrintString "Добежал")))
    (else
      (Development|PrintString "Error: Index out of bounds")))
  (AI|BehaviorTree|FinishExecute (and (< _destinationindex (Utilities|Array|Length _outactors)) (>= _destinationindex 0))))